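; Anim notify for Tiyanak enemy animations that plays footstep sounds according to the surface under a visibility sphere trace from the owner.
; The trace ends at the raw up vector, used as a world position rather than an offset from the owner.
; Metal plays the player's metal footsteps, while Carpet, Rock and Wood share the Tiyanak sound, both at the hit location.
; The GetActorOfClass lookup result is unused.
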(fn ReceivedNotify
  (params (MeshComp :type Skeletal%20Mesh%20Component%20Object%20Reference) (Animation :type Anim%20Sequence%20Base%20Object%20Reference) (EventReference :type Anim%20Notify%20Event%20Reference%20Structure%20%28by%20ref%29))
  (bind _returnvalue (Components|GetOwner MeshComp))
  (Actor|GetActorOfClass "/Game/CAPSTN1/Enemy/AI/Enemies/S_Enemy_Tiyanak.S_Enemy_Tiyanak_C")
  (bind (_outhit _returnvalue_2) (Collision|SphereTraceByChannel (Transformation|GetActorLocation _returnvalue) (Transformation|GetActorUpVector _returnvalue) 0.0 "TraceTypeQuery1" false (Utilities|Array|MakeArray _returnvalue) "None"))
  (if _returnvalue_2
    (switch Utilities|FlowControl|Switch|SwitchonEPhysicalSurface (Collision|GetSurfaceType _outhit)
      (:SurfaceType1
        (Audio|PlaySoundatLocation "/Game/CAPSTN1/CAPSTN_Assets/Sounds/SoundCues/Tiyanakfootsteps.Tiyanakfootsteps" (.Location (Collision|BreakHitResult _outhit)) "0, 0, 0" 1.0 1.0 0.0 0 0 0 0 :!label _label))
      (:SurfaceType4
        (Audio|PlaySoundatLocation "/Game/CAPSTN1/CAPSTN_Assets/Sounds/Player/PlayerMetalFootsteps.PlayerMetalFootsteps" (.Location (Collision|BreakHitResult _outhit)) "0, 0, 0" 1.0 1.0 0.0 0 0 0 0))
      (:SurfaceType5
        (goto _label))
      (:SurfaceType7
        (goto _label)))
    (return false)))